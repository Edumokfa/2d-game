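; Paper2D door Blueprint that drives its flipbook animation from the player's position.
; BeginPlay starts the flipbook from the beginning.
; Every Tick polls player 0's location against a hardcoded world-space X range and minimum Z height, with no trigger volume.
; Inside that zone the flipbook plays with looping disabled, and outside it playback stops.
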(event `self.ReceiveTick`
  (params (DeltaSeconds :type "Float (single-precision)"))
  (bind _x (.x (`self.K2_GetActorLocation` (`GameplayStatics.GetPlayerCharacter` 0))))
  (if (and (and (> _x 5357.0) (< _x 5580.0)) (> (.z (`self.K2_GetActorLocation` (`GameplayStatics.GetPlayerCharacter` 0))) 240.0))
    (`PaperFlipbookComponent.Play` (`self.PaperFlipbook`))
    (`PaperFlipbookComponent.SetLooping` (`self.PaperFlipbook`) false)
    (else
      (`PaperFlipbookComponent.Stop` (`self.PaperFlipbook`)))))

(event `self.ReceiveBeginPlay`
  (`PaperFlipbookComponent.PlayFromStart` (`self.PaperFlipbook`)))

(fn `UserConstructionScript`)